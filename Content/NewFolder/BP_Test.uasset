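; BP_Test is a debug test actor that compares stepped yaw-and-move placement against a single combined move.
; TestAngles loops over Horizontal, adding Angle yaw and a fixed forward step, teleless-moving the actor and drawing debug spheres and lines.
; It then rotates from the initial transform by the total angle, moves the full distance in one jump, and marks that endpoint in red.
; TestPositionGeneration is an empty stub.
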(event `TestAngles`
  (bind _returnvalue_location (`KismetMathLibrary.BreakTransform` (`self.GetTransform`)))
  (bind _returnvalue (`self.GetTransform`))
  (bind _horizontal (`self.Horizontal`))
  (bind (_newvar_location _newvar_rotation) (`KismetMathLibrary.BreakTransform` (`self.NewVar`)))
  (bind _initialtransform_location (`KismetMathLibrary.BreakTransform` (`self.InitialTransform`)))
  (bind (_newvar_location_2 _newvar_rotation_2) (`KismetMathLibrary.BreakTransform` (`self.NewVar`)))
  (bind (_newvar_location_3 _newvar_rotation_3 _newvar_scale) (`KismetMathLibrary.BreakTransform` (`self.NewVar`)))
  (bind (_newvar_location_4 _newvar_rotation_4 _newvar_scale_2) (`KismetMathLibrary.BreakTransform` (`self.NewVar`)))
  (bind (_newvar_location_5 _newvar_rotation_5 _newvar_scale_3) (`KismetMathLibrary.BreakTransform` (`self.NewVar`)))
  (bind (_newvar_location_6 _newvar_rotation_6 _newvar_scale_4) (`KismetMathLibrary.BreakTransform` (`self.NewVar`)))
  (set `self.InitialTransform` _returnvalue)
  (set `self.NewVar` _returnvalue)
  (for _ (range (+ _horizontal 1))
    (set `self.NewVar` (`KismetMathLibrary.MakeTransform` _newvar_location_5 (`KismetMathLibrary.ComposeRotators` _newvar_rotation_2 (`KismetMathLibrary.MakeRotator` 0.0 0.0 (`self.Angle`))) _newvar_scale_3))
    (bind _output_get (set `self.NewVar` (`KismetMathLibrary.MakeTransform` (+ _newvar_location_6 (* (`self.GetActorForwardVector`) 48.0)) _newvar_rotation_6 _newvar_scale_4)))
    (`KismetSystemLibrary.DrawDebugSphere` (.location _output_get) 5.0 12 (struct :`R` 1.0 :`G` 1.0 :`B` 1.0 :`A` 1.0) 15.0 1.0)
    (`KismetSystemLibrary.DrawDebugLine` _returnvalue_location (.location _output_get) (struct) 15.0 1.0)
    (`self.K2_SetActorTransform` (`self.NewVar`)))
  (set `self.NewVar` (`self.InitialTransform`))
  (set `self.NewVar` (`KismetMathLibrary.MakeTransform` _newvar_location_4 (`KismetMathLibrary.ComposeRotators` _newvar_rotation (`KismetMathLibrary.MakeRotator` 0.0 0.0 (`KismetMathLibrary.Conv_IntToDouble` (* _horizontal (`self.Angle`))))) _newvar_scale_2))
  (`self.K2_SetActorTransform` (`self.NewVar`))
  (bind _output_get_2 (set `self.NewVar` (`KismetMathLibrary.MakeTransform` (+ _newvar_location_3 (* (`self.GetActorForwardVector`) (* _horizontal 48))) _newvar_rotation_3 _newvar_scale)))
  (`KismetSystemLibrary.DrawDebugSphere` (.location _output_get_2) 5.0 12 (struct :`R` 1.0 :`G` 0.125397 :`A` 1.0) 15.0 1.0)
  (`KismetSystemLibrary.DrawDebugLine` _initialtransform_location (.location _output_get_2) (struct :`R` 1.0 :`G` 0.099749 :`A` 1.0) 15.0 1.0)
  (`self.K2_SetActorTransform` (`self.NewVar`)))

(event `TestPositionGeneration`)

(fn `UserConstructionScript`)